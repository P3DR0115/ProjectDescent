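; CameraForTrack is a camera actor that travels along the spline of a referenced track, starting at BeginPlay when ActiveCamera is set.
; A timeline, rate-scaled by Duration and started at CameraStartOffset, drives a curve that maps to distance along the spline, setting location and rotation.
; Each timeline update also flips PlayerTurn and calls a Delay that leads nowhere.
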(event `self.ReceiveBeginPlay`
  (if (`self.ActiveCamera`)
    (`self.MoveCamera`)))

(event `MoveCamera`
  (bind _returnvalue (`KismetMathLibrary.Lerp` 0.0 (`SplineComponent.GetSplineLength` (`/Game/Blueprints/Game/CameraTrack.Track` (`self.TrackRef`))) (`self.Curve`)))
  (`TimelineComponent.SetPlayRate` (`self.CameraMover2`) (/ 1.0 (`self.Duration`)))
  (`TimelineComponent.SetNewTime` (`self.CameraMover2`) (`self.CameraStartOffset`))
  (bind (_direction _begincurve) (`Timeline|CameraMover2`)
    (:`Update`
      (set `self.Curve` _begincurve)
      (`self.K2_SetActorLocationAndRotation` (`SplineComponent.GetLocationAtDistanceAlongSpline` (`/Game/Blueprints/Game/CameraTrack.Track` (`self.TrackRef`)) _returnvalue "World") (`SplineComponent.GetRotationAtDistanceAlongSpline` (`/Game/Blueprints/Game/CameraTrack.Track` (`self.TrackRef`)) _returnvalue "World"))
      (if (`self.PlayerTurn`)
        (set `self.PlayerTurn` false)
        (else
          (set `self.PlayerTurn` true)))
      (`KismetSystemLibrary.Delay` (`self.Duration`)))))

(fn `UserConstructionScript`)