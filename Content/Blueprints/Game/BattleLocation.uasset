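; BattleLocation is an actor that starts a battle when play begins; its random-chance check (0 to 2, under 3) always passes.
; It stops and disables player input, shows the BattleHUD_Fade widget and clears the BattleTrigger timer.
; After a short delay, it spawns a battle manager at the position of the BattleLocation found by class lookup, then switches the player's view to it.
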(event `self.ReceiveBeginPlay`
  (bind _returnvalue (`GameplayStatics.GetPlayerController` 0))
  (if (< (`KismetMathLibrary.RandomIntegerInRange` 0 2) 3)
    (`Controller.StopMovement` _returnvalue)
    (`self.DisableInput` _returnvalue)
    (bind _returnvalue_2 (`|CreateWidget` "/Game/Blueprints/Widgets/BattleHUD_Fade.BattleHUD_Fade_C" _returnvalue))
    (`UserWidget.AddToViewport` _returnvalue_2 0)
    (bind _returnvalue_3 (`GameplayStatics.GetActorOfClass` "BattleLocation_C"))
    (`KismetSystemLibrary.K2_ClearTimer` null "BattleTrigger")
    (`KismetSystemLibrary.Delay` 1.5)
    (bind _returnvalue_4 (`|SpawnActorFromClass` "/Game/Blueprints/Game/BattleManager.BattleManager_C" (`KismetMathLibrary.MakeTransform` (`SceneComponent.K2_GetComponentLocation` (`Actor.RootComponent` _returnvalue_3))) "Undefined" "OverrideRootScale" null null))
    (bind _output_get (set `self.BattleManagerRef` _returnvalue_4))
    (`PlayerController.SetViewTargetWithBlend` (`GameplayStatics.GetPlayerController` 0) _output_get 0.0 "VTBlend_Linear" 0.0 false)))

(fn `UserConstructionScript`)