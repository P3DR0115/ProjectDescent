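; CameraMover is an unfinished helper that moves the top-down player character's camera while a PlayerTurn flag is set.
; On BeginPlay it caches player 0's pawn as a TopDownCharacter.
; Each tick during the turn it stores delta time and the camera's location, then sets the camera component to the world origin, using neither stored value.
; Nothing in this graph sets PlayerTurn.
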(event `self.ReceiveBeginPlay`
  (bind _astop_down_character (cast `/Game/TopDownCPP/Blueprints/TopDownCharacter` (`GameplayStatics.GetPlayerCharacter` 0)))
  (set `self.PlayerRef` _astop_down_character))

(event `self.ReceiveTick`
  (params (DeltaSeconds :type "Float (single-precision)"))
  (bind _topdowncameracomponent (`ProjectDescentCharacter.TopDownCameraComponent` (`self.PlayerRef`)))
  (if (`self.PlayerTurn`)
    (set `self.NewVar_0` DeltaSeconds)
    (set `self.CurrentCamLocation` (`SceneComponent.K2_GetComponentLocation` _topdowncameracomponent))
    (`SceneComponent.K2_SetWorldLocation` _topdowncameracomponent (0.0 0.0 0.0) false false)))

(fn `UserConstructionScript`)