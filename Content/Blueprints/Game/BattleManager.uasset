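; Turn-based battle manager that spawns three enemies and three party members, creates the battle HUDs and runs the turn loop.
; A single adjacent-swap pass over the combatants roughly orders them by descending Initiative, then each receives its turn index.
; Enemy turns attack a random party member, play a timeline nudge and advance the turn; player turns use the ADAM widget, created on first need.
; The battle camera intro is not triggered.
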(event `CreateADAM`
  (bind _returnvalue (`|CreateWidget` "/Game/Blueprints/Widgets/BattleHUD_ADAM.BattleHUD_ADAM_C" null self))
  (bind _output_get (set `self.AdamWidgetRef` _returnvalue))
  (`UserWidget.AddToViewport` _output_get 0))

(event `self.ReceiveBeginPlay`
  (`self.SpawnEnemies`)
  (`self.SpawnPlayers`)
  (`self.TurnCalculation`)
  (bind _returnvalue (`|CreateWidget` "/Game/Blueprints/Widgets/MainHUD.MainHUD_C" null self))
  (bind _output_get (set `self.MainHUDRef` _returnvalue))
  (`UserWidget.AddToViewport` _output_get 0)
  (`self.DetermineEnemyTurn`))

(event `SpawnBattleCamera`
  (bind _returnvalue (`|SpawnActorFromClass` "/Game/Blueprints/Game/BattleCamera.BattleCamera_C" (`self.GetTransform`) "Undefined" "OverrideRootScale" null null))
  (bind _output_get (set `self.BattleCam` _returnvalue))
  (`KismetSystemLibrary.Delay` 0.2)
  (`PlayerController.SetViewTargetWithBlend` (`GameplayStatics.GetPlayerController` 0) _output_get 1.5 "VTBlend_Linear" 0.0 false)
  (`KismetSystemLibrary.Delay` 4.5)
  (bind _returnvalue_2 (`|CreateWidget` "/Game/Blueprints/Widgets/MainHUD.MainHUD_C" null self))
  (bind _output_get_2 (set `self.MainHUDRef` _returnvalue_2))
  (`UserWidget.AddToViewport` _output_get_2 0)
  (`self.DetermineEnemyTurn`))

(event `SpawnEnemies`
  (bind _returnvalue (`|SpawnActorFromClass` "/Game/Blueprints/Game/EnemyChars/MyEnemyTest_CharBP.MyEnemyTest_CharBP_C" (`SceneComponent.K2_GetComponentToWorld` (`self.SpawnE1`)) "Undefined" "OverrideRootScale" null null))
  (set `self.Enemy1` _returnvalue)
  (switch `int` (`KismetMathLibrary.RandomIntegerInRange` 0)
    (:`0`
      (bind _returnvalue_2 (`|SpawnActorFromClass` "/Game/Blueprints/Game/EnemyChars/MyEnemyTest_CharBP.MyEnemyTest_CharBP_C" (`SceneComponent.K2_GetComponentToWorld` (`self.SpawnE2`)) "Undefined" "OverrideRootScale" null null))
      (set `self.Enemy2` _returnvalue_2)
      (switch `int` (`KismetMathLibrary.RandomIntegerInRange` 0)
        (:`0`
          (bind _returnvalue_3 (`|SpawnActorFromClass` "/Game/Blueprints/Game/EnemyChars/MyEnemyTest_CharBP.MyEnemyTest_CharBP_C" (`SceneComponent.K2_GetComponentToWorld` (`self.SpawnE3`)) "Undefined" "OverrideRootScale" null null))
          (set `self.Enemy3` _returnvalue_3))))))

(event `SpawnPlayers`
  (bind _returnvalue (`|SpawnActorFromClass` "/Game/Blueprints/Game/PlayerChars/MyRogue_CharBP.MyRogue_CharBP_C" (`SceneComponent.K2_GetComponentToWorld` (`self.SpawnPM1`)) "Undefined" "OverrideRootScale" null null))
  (set `self.PlayerMember1` _returnvalue)
  (bind _returnvalue_2 (`|SpawnActorFromClass` "/Game/Blueprints/Game/PlayerChars/MyRogue_CharBP.MyRogue_CharBP_C" (`SceneComponent.K2_GetComponentToWorld` (`self.SpawnPM2`)) "Undefined" "OverrideRootScale" null null))
  (set `self.PlayerMember2` _returnvalue_2)
  (bind _returnvalue_3 (`|SpawnActorFromClass` "/Game/Blueprints/Game/PlayerChars/MyRogue_CharBP.MyRogue_CharBP_C" (`SceneComponent.K2_GetComponentToWorld` (`self.SpawnPM3`)) "Undefined" "OverrideRootScale" null null))
  (set `self.PlayerMember3` _returnvalue_3))

(event `TurnCalculation`
  (bind _playermember1 (`self.PlayerMember1`))
  (bind _playermember3 (`self.PlayerMember3`))
  (bind _combatantsinorder (`self.CombatantsInOrder`))
  (bind _enemy1 (`self.Enemy1`))
  (bind _playermember2 (`self.PlayerMember2`))
  (bind _enemy2 (`self.Enemy2`))
  (bind _enemy3 (`self.Enemy3`))
  (`|ExecutionSequence`
    (:`then_0`
      (`/Engine/EditorBlueprintResources/StandardMacros.IsValid` _enemy1
        (:`Is Valid`
          (`KismetArrayLibrary.Array_Add` (`self.EnemyArray`) _enemy1)
          (`KismetArrayLibrary.Array_Add` (`self.CombatantsInOrder`) _enemy1))))
    (:`then_1`
      (`/Engine/EditorBlueprintResources/StandardMacros.IsValid` _enemy2
        (:`Is Valid`
          (`KismetArrayLibrary.Array_Add` (`self.EnemyArray`) _enemy2)
          (`KismetArrayLibrary.Array_Add` (`self.CombatantsInOrder`) _enemy2))))
    (:`then_2`
      (`/Engine/EditorBlueprintResources/StandardMacros.IsValid` _enemy3
        (:`Is Valid`
          (`KismetArrayLibrary.Array_Add` (`self.EnemyArray`) _enemy3)
          (`KismetArrayLibrary.Array_Add` (`self.CombatantsInOrder`) _enemy3))))
    (:`then_3`
      (`/Engine/EditorBlueprintResources/StandardMacros.IsValid` _playermember1
        (:`Is Valid`
          (`KismetArrayLibrary.Array_Add` (`self.PlayerPartyArray`) _playermember1)
          (`KismetArrayLibrary.Array_Add` (`self.CombatantsInOrder`) _playermember1)
          (`/Engine/EditorBlueprintResources/StandardMacros.IsValid` _playermember2
            (:`Is Valid`
              (`KismetArrayLibrary.Array_Add` (`self.PlayerPartyArray`) _playermember2)
              (`KismetArrayLibrary.Array_Add` (`self.CombatantsInOrder`) _playermember2)
              (`/Engine/EditorBlueprintResources/StandardMacros.IsValid` _playermember3
                (:`Is Valid`
                  (`KismetArrayLibrary.Array_Add` (`self.PlayerPartyArray`) _playermember3)
                  (`KismetArrayLibrary.Array_Add` (`self.CombatantsInOrder`) _playermember3))))))))
    (:`then_4`
      (for (_array_element _array_index) (`self.CombatantsInOrder`)
        (bind _returnvalue (`TurnBasedCharacter.GetTurnStruct` _array_element))
        (bind _returnvalue_2 (+ _array_index 1))
        (if (`KismetArrayLibrary.Array_IsValidIndex` _combatantsinorder _returnvalue_2)
          (bind _returnvalue_3 (`TurnBasedCharacter.GetTurnStruct` (`|GetArrayItem` _combatantsinorder _returnvalue_2)))
          (if (not (> (break `TurnStruct` _returnvalue) (break `TurnStruct` _returnvalue_3)))
            (`KismetArrayLibrary.Array_Swap` (`self.CombatantsInOrder`) _array_index _returnvalue_2)))))
    (:`then_5`
      (for (_array_element_2 _array_index_2) (`self.CombatantsInOrder`)
        (`TurnBasedCharacter.SetTurnOrder` _array_element_2 _array_index_2)))))

(event `NextTurn`
  (bind _turnindex (`self.TurnIndex`))
  (if (>= _turnindex (- (`KismetArrayLibrary.Array_Length` (`self.CombatantsInOrder`)) 1))
    (bind _output_get (set `self.TurnIndex` 0))
    (`KismetSystemLibrary.PrintString` (`KismetStringLibrary.Concat_StrStr` "TurnIndex: " (`KismetStringLibrary.Conv_IntToString` _output_get)))
    (`self.DetermineEnemyTurn`)
    (else
      (bind _output_get_2 (set `self.TurnIndex` (+ _turnindex 1)))
      (`KismetSystemLibrary.PrintString` (`KismetStringLibrary.Concat_StrStr` "TurnIndex: " (`KismetStringLibrary.Conv_IntToString` _output_get_2)))
      (`self.DetermineEnemyTurn`))))

(event `DetermineEnemyTurn`
  (bind _adamwidgetref (`self.AdamWidgetRef`))
  (bind _output (`|GetArrayItem` (`self.CombatantsInOrder`) (`self.TurnIndex`)))
  (if (`KismetMathLibrary.ClassIsChildOf` (`GameplayStatics.GetObjectClass` _output) "/Script/ProjectDescent.EnemyBaseChar")
    (`self.EnemyTurn`)
    (else
      (`/Engine/EditorBlueprintResources/StandardMacros.IsValid` _adamwidgetref
        (:`Is Valid`
          (`TurnBasedCharacter.BeginTurn` _output)
          (`/Game/Blueprints/Widgets/BattleHUD_ADAM.PlayFadeIn` _adamwidgetref))
        (:`Is Not Valid`
          (`self.CreateADAM`))))))

(event `EnemyTurn`
  (bind _playerpartyarray (`self.PlayerPartyArray`))
  (bind _asenemy_test_char (cast `EnemyTest_Char` (`|GetArrayItem` (`self.CombatantsInOrder`) (`self.TurnIndex`))))
  (bind _output_get (set `self.SelectedTarget` (`KismetMathLibrary.RandomIntegerInRange` 0 (- (`KismetArrayLibrary.Array_Length` _playerpartyarray) 1))))
  (bind _output (`|GetArrayItem` _playerpartyarray _output_get))
  (`EnemyBaseChar.TurnIntent` _asenemy_test_char _output)
  (bind (_statsstruct_turnstruct _statsstruct_maxhealthpoints _statsstruct_currenthealthpoints) (break `StatsStruct` (`TurnBasedCharacter.StatsStruct` _output)))
  (`KismetSystemLibrary.PrintString` (`KismetStringLibrary.Concat_StrStr` (`KismetStringLibrary.Conv_IntToString` (`self.SelectedTarget`)) " (player) was attacked: " (`KismetStringLibrary.Conv_IntToString` _statsstruct_currenthealthpoints) " HP remaining"))
  (`Timeline|MiniAttackMove`
    (:`Update`
      (`self.ActionMiniAnim` _asenemy_test_char)
      (`KismetSystemLibrary.Delay` 1.0)
      (`self.ActionMiniAnim` _asenemy_test_char true)
      (`self.NextTurn`))))

(fn `ActionMiniAnim`
  (params (CharacterToAnim :type "TurnBasedCharacter Object Reference") (Reverse :type Boolean))
  (bind (_returnvalue_x _returnvalue_y _returnvalue_z) (`KismetMathLibrary.BreakVector` (`self.K2_GetActorLocation` (`local.CharacterToAnim`))))
  (bind (_returnvalue_x_2 _returnvalue_y_2 _returnvalue_z_2) (`KismetMathLibrary.BreakVector` (`self.K2_GetActorLocation` (`local.CharacterToAnim`))))
  (if Reverse
    (bind _result (`/Engine/EditorBlueprintResources/StandardMacros.NegateFloat` (`self.AnimMoveValue`))
      (:`  `
        (`self.K2_SetActorLocation` (`local.CharacterToAnim`) (`KismetMathLibrary.MakeVector` (+ _returnvalue_x_2 _result) _returnvalue_y_2 _returnvalue_z_2) false false)))
    (else
      (`self.K2_SetActorLocation` (`local.CharacterToAnim`) (`KismetMathLibrary.MakeVector` (+ _returnvalue_x (`self.AnimMoveValue`)) _returnvalue_y _returnvalue_z) false false))))

(fn `GetCurrentCombatant`
  (returns (Character :type "TurnBasedCharacter Object Reference"))
  (return (`|GetArrayItem` (`self.CombatantsInOrder`) (`self.TurnIndex`))))

(fn `UserConstructionScript`)